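; Tank Blueprint that handles player camera aiming and switching between a large and a small cannon.
; On BeginPlay it passes the Cannon and SmallCannon components to SetBarrelReference.
; Aim axis inputs add local yaw to an azimuth gimbal and local pitch to the spring arm, keeping the two rotations on separate components.
; The ChangeCannon input calls the function of the same name, whose logic lives outside these graphs.
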(event `self.ReceiveBeginPlay`
  (`self.SetBarrelReference` (`self.Cannon`) (`self.Small_Cannon`)))

(event `InputAxis|AimAzumuth`
  (params (AxisValue :type "Float (single-precision)"))
  (`SceneComponent.K2_AddLocalRotation` (`self.AzumuthGimbal`) (`KismetMathLibrary.MakeRotator` 0.0 0.0 AxisValue) false false))

(event `InputAxis|AimElevation`
  (params (AxisValue :type "Float (single-precision)"))
  (`SceneComponent.K2_AddLocalRotation` (`self.SpringArm`) (`KismetMathLibrary.MakeRotator` 0.0 AxisValue) false false))

(event `InputAction|ChangeCannon`
  (params (Key :type "Key Structure"))
  (:`Pressed`
    (`self.ChangeCannon`)))

(fn `UserConstructionScript`)